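; Player controller for a ball-and-score game that creates the GameGui HUD and tracks score and remaining balls.
; Score updates refresh the HUD and award an extra ball with a sound at a threshold that multiplies after each award.
; Removing a ball, also done once at setup, pauses the game when none remain.
; It forces fullscreen 1080p after startup or on Alt+Enter, and Escape quits.
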(event `self.ReceiveBeginPlay`
  (`|ExecutionSequence`
    (:`then_0`
      (bind _returnvalue (`|CreateWidget` "/Game/GameGui.GameGui_C" self))
      (`UserWidget.AddToViewport` _returnvalue)
      (bind _asgame_gui (cast `/Game/GameGui` _returnvalue))
      (set `self.GameGui` _asgame_gui))
    (:`then_1`
      (`KismetSystemLibrary.Delay` 0.05)
      (`KismetSystemLibrary.ExecuteConsoleCommand` "r.FullscreenMode 1" :!label _label)
      (`KismetSystemLibrary.ExecuteConsoleCommand` "SETRES 1920x1080f"))
    (:`then_2`
      (`self.setDefaults`))))

(event `Key|Alt+Enter`
  (:`Pressed`
    (goto _label)))

(event `Key|Escape`
  (:`Pressed`
    (`KismetSystemLibrary.QuitGame` null "Quit")))

(event `setDefaults`
  (`self.updateScore` 0)
  (`self.removeBall`))

(fn `ExtraBall`
  (set `self.currentBalls` (+ (`self.currentBalls`) 1))
  (set `self.nextExtraBallScore` (`KismetMathLibrary.FFloor` (* (`self.nextExtraBallScore`) 2.5)))
  (`GameplayStatics.PlaySoundAtLocation` "/Game/ExtraBall.ExtraBall")
  (`TextBlock.SetText` (`/Game/GameGui.ballsTxt` (`self.GameGui`)) (`KismetTextLibrary.Conv_StringToText` (`KismetStringLibrary.Conv_IntToString` (`self.currentBalls`)))))

(fn `removeBall`
  (bind _returnvalue (- (`self.currentBalls`) 1))
  (`TextBlock.SetText` (`/Game/GameGui.ballsTxt` (`self.GameGui`)) (`KismetTextLibrary.Conv_StringToText` (`KismetStringLibrary.Conv_IntToString` _returnvalue)))
  (if (>= _returnvalue 0)
    (set `self.currentBalls` _returnvalue)
    (else
      (`GameplayStatics.SetGamePaused` true)
      (set `self.currentBalls` 0))))

(fn `updateScore`
  (params (additionalPoints :type Integer))
  (bind _returnvalue (+ (`self.currentScore`) additionalPoints))
  (`TextBlock.SetText` (`/Game/GameGui.scoreTxt` (`self.GameGui`)) (`KismetTextLibrary.Conv_StringToText` (`KismetStringLibrary.Conv_IntToString` _returnvalue)))
  (set `self.currentScore` _returnvalue)
  (if (>= (`self.currentScore`) (`self.nextExtraBallScore`))
    (`self.ExtraBall`)))

(fn `UserConstructionScript`)