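; Player controller for a pinball game that manages score, balls, the start, HUD and end-screen widgets, plus fullscreen and quit keys.
; BeginPinballGame swaps the start screen for the HUD and fires the game-start dispatcher.
; Score updates award extra balls at a multiplicatively growing threshold, while removing a ball with none left shows the end screen and pauses.
; Restarting resets score and balls but not that threshold.
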(event `self.ReceiveBeginPlay`
  (`|ExecutionSequence`
    (:`then_0`
      (bind _returnvalue (`|CreateWidget` "/Game/NewFolder/StartGUI.StartGUI_C" self))
      (`UserWidget.AddToViewport` _returnvalue)
      (set `self.Start GUI` _returnvalue)
      (`GameplayStatics.PlaySoundAtLocation` "/Game/startgame.startgame"))))

(event `Key|Alt+Enter` :paused true
  (:`Pressed`
    (`KismetSystemLibrary.ExecuteConsoleCommand` "r.FullscreenMode 1")
    (`KismetSystemLibrary.ExecuteConsoleCommand` "SETRES 1920x1080f")))

(event `Key|Escape` :paused true
  (:`Pressed`
    (`KismetSystemLibrary.QuitGame` null "Quit")))

(event `BeginPinballGame`
  (`|ExecutionSequence`
    (:`then_0`
      (bind _returnvalue (`|CreateWidget` "/Game/GameGui.GameGui_C" self))
      (`UserWidget.AddToViewport` _returnvalue)
      (bind _asgame_gui (cast `/Game/GameGui` _returnvalue))
      (set `self.Game Gui` _asgame_gui))
    (:`then_1`
      (`self.setDefaults`))
    (:`then_2`
      (`GameplayStatics.PlaySoundAtLocation` "/Game/start.start"))
    (:`then_3`
      (if (`KismetSystemLibrary.IsValid` (`self.Start GUI`))
        (`Widget.RemoveFromParent` (`self.Start GUI`))
        (`self.GameStartDispatcher`)))))

(event `setDefaults`
  (`self.updateScore` 0))

(fn `ExtraBall`
  (set `self.currentBalls` (+ (`self.currentBalls`) 1))
  (set `self.nextExtraBallScore` (`KismetMathLibrary.FFloor` (* (`self.nextExtraBallScore`) 2.5)))
  (`GameplayStatics.PlaySoundAtLocation` "/Game/ExtraBall.ExtraBall")
  (`self.UpdateGui`))

(fn `removeBall`
  (bind _returnvalue (- (`self.currentBalls`) 1))
  (if (>= _returnvalue 0)
    (set `self.currentBalls` _returnvalue)
    (`self.UpdateGui`)
    (else
      (set `self.currentBalls` 0)
      (bind _returnvalue_2 (`|CreateWidget` "/Game/EndGui.EndGui_C" self))
      (`UserWidget.AddToViewport` _returnvalue_2)
      (set `self.EndGui` _returnvalue_2)
      (`self.UpdateGui`)
      (`GameplayStatics.SetGamePaused` true))))

(fn `Reset Game`
  (set `self.currentScore` 0)
  (set `self.currentBalls` 3)
  (`self.UpdateGui`))

(fn `RestartGame`
  (if (`KismetSystemLibrary.IsValid` (`self.EndGui`))
    (`Widget.RemoveFromParent` (`self.EndGui`))
    (`self.Reset Game`)
    (`GameplayStatics.SetGamePaused` false)))

(fn `UpdateGui`
  (`TextBlock.SetText` (`/Game/GameGui.scoreTxt` (`self.Game Gui`)) (`KismetTextLibrary.Conv_StringToText` (`KismetStringLibrary.Conv_IntToString` (`self.currentScore`))))
  (`TextBlock.SetText` (`/Game/GameGui.ballsTxt` (`self.Game Gui`)) (`KismetTextLibrary.Conv_StringToText` (`KismetStringLibrary.Conv_IntToString` (`self.currentBalls`)))))

(fn `updateScore`
  (params (additionalPoints :type Integer))
  (set `self.currentScore` (+ (`self.currentScore`) additionalPoints))
  (`self.UpdateGui`)
  (if (>= (`self.currentScore`) (`self.nextExtraBallScore`))
    (`self.ExtraBall`)))

(fn `UserConstructionScript`)